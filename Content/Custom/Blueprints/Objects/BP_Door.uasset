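; BP_Door is an interactable door that the player opens by pressing E near it.
; Entering the trigger while the door is closed enables input and shows a prompt widget with the interaction text.
; Pressing E plays a timeline that sets the Open flag and drives the door's relative yaw, with no closing logic.
; Leaving the trigger disables input and removes the prompt after a short delay.
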(event `self.Trigger.OnComponentBeginOverlap`
  (params (OverlappedComponent :type "PrimitiveComponent Object Reference") (OtherActor :type "Actor Object Reference") (OtherComp :type "PrimitiveComponent Object Reference") (OtherBodyIndex :type Integer) (bFromSweep :type Boolean) (SweepResult :type "HitResult Structure (by ref)"))
  (bind _returnvalue (`GameplayStatics.GetPlayerController` 0))
  (if (not (`self.Open`))
    (`self.EnableInput` _returnvalue)
    (bind _returnvalue_2 (`|CreateWidget` "/Game/Custom/HUD/Prompts/Prompt_Base.Prompt_Base_C" _returnvalue))
    (set `/Game/Custom/HUD/Prompts/Prompt_Base.Interaction Text` (`self.Interaction Text`) _returnvalue_2)
    (`UserWidget.AddToViewport` _returnvalue_2 0)))

(event `self.Trigger.OnComponentEndOverlap`
  (params (OverlappedComponent :type "PrimitiveComponent Object Reference") (OtherActor :type "Actor Object Reference") (OtherComp :type "PrimitiveComponent Object Reference") (OtherBodyIndex :type Integer))
  (`self.DisableInput` (`GameplayStatics.GetPlayerController` 0))
  (`KismetSystemLibrary.Delay` 1.0)
  (`Widget.RemoveFromParent` (stale `self.Trigger.OnComponentBeginOverlap` _returnvalue_2)))

(event `Key|E`
  (params (Key :type "Key Structure"))
  (:`Pressed`
    (bind (_direction _rotation) (`Timeline|DoorTimeLine` :`NewTime` 3.0)
      (:`Update`
        (set `self.Open` true)
        (`SceneComponent.K2_SetRelativeRotation` (`self.Door`) (`KismetMathLibrary.MakeRotator` 0.0 0.0 _rotation) false false)))))

(fn `UserConstructionScript`)