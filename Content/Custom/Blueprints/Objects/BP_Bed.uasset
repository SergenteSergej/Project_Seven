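; BP_Bed is an interactable bed that puts the player to sleep.
; Overlapping BedTrigger enables input and shows a prompt widget unless already sleeping; leaving disables input and removes it.
; Pressing E fades the camera to a held black, disables the overlapping actor's input, sets IsSleeping and removes the prompt.
; After a delay matching the fade, it displays a Prompt_Base widget with SafetyNotice text.
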(event `self.BedTrigger.OnComponentBeginOverlap`
  (params (OverlappedComponent :type "PrimitiveComponent Object Reference") (OtherActor :type "Actor Object Reference") (OtherComp :type "PrimitiveComponent Object Reference") (OtherBodyIndex :type Integer) (bFromSweep :type Boolean) (SweepResult :type "HitResult Structure (by ref)"))
  (bind _returnvalue (`GameplayStatics.GetPlayerController` 0))
  (if (not (`self.IsSleeping`))
    (`self.EnableInput` _returnvalue)
    (bind _returnvalue_2 (`|CreateWidget` "/Game/Custom/HUD/Prompts/Prompt_Base.Prompt_Base_C" _returnvalue))
    (set `/Game/Custom/HUD/Prompts/Prompt_Base.Interaction Text` (`self.Bed Prompt`) _returnvalue_2)
    (`UserWidget.AddToViewport` _returnvalue_2 0)))

(event `self.BedTrigger.OnComponentEndOverlap`
  (params (OverlappedComponent :type "PrimitiveComponent Object Reference") (OtherActor :type "Actor Object Reference") (OtherComp :type "PrimitiveComponent Object Reference") (OtherBodyIndex :type Integer))
  (`self.DisableInput` (`GameplayStatics.GetPlayerController` 0))
  (`Widget.RemoveFromParent` (stale `self.BedTrigger.OnComponentBeginOverlap` _returnvalue_2)))

(event `Key|E`
  (params (Key :type "Key Structure"))
  (:`Pressed`
    (`PlayerCameraManager.StartCameraFade` :`self` (`GameplayStatics.GetPlayerCameraManager` 0) :`ToAlpha` 1.0 :`Duration` 2.0 :`bHoldWhenFinished` true)
    (`self.DisableInput` (stale `self.BedTrigger.OnComponentBeginOverlap` OtherActor) (`GameplayStatics.GetPlayerController` 0))
    (set `self.IsSleeping` true)
    (`Widget.RemoveFromParent` (stale `self.BedTrigger.OnComponentBeginOverlap` _returnvalue_2))
    (`KismetSystemLibrary.Delay` 2.0)
    (bind _returnvalue (`|CreateWidget` "/Game/Custom/HUD/Prompts/Prompt_Base.Prompt_Base_C"))
    (set `/Game/Custom/HUD/Prompts/Prompt_Base.Interaction Text` (`self.Safety Notice`) _returnvalue)
    (`UserWidget.AddToViewport` _returnvalue 0)))

(fn `UserConstructionScript`)